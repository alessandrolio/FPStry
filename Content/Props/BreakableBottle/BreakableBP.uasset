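; Breakable potion bottle prop that swaps itself for a destructible version when it moves fast.
; Tick checks the PotionC component's speed and, once past a threshold, a DoOnce spawns DestructiblePotionCAttore at its transform.
; The spawned destructible gets an impulse from the component hit event's data, the original component is destroyed, and temporary smoke plays at the hit location.
; The hit event itself triggers no logic.
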(event `self.ReceiveBeginPlay`)

(event `self.ReceiveTick`
  (params (DeltaSeconds :type "Float (single-precision)"))
  (if (> (`KismetMathLibrary.VSize` (`SceneComponent.GetComponentVelocity` (`self.PotionC`))) 2500.0)
    (`/Engine/EditorBlueprintResources/StandardMacros.DoOnce` false
      (:`Completed`
        (bind _returnvalue (`|SpawnActorFromClass` "/Game/Props/BreakableBottle/DestructiblePotionCAttore.DestructiblePotionCAttore_C" (`SceneComponent.K2_GetComponentToWorld` (`self.PotionC`)) "Undefined" "OverrideRootScale" null null))
        (`|ExecutionSequence`
          (:`then_0`
            (bind (_bblockinghit _binitialoverlap _time _distance _location) (`GameplayStatics.BreakHitResult` (stale `self.PotionC.OnComponentHit` Hit)))
            (`PrimitiveComponent.AddImpulseAtLocation` (`/Game/Props/BreakableBottle/DestructiblePotionCAttore.Destructible` _returnvalue) (stale `self.PotionC.OnComponentHit` NormalImpulse) _location "None"))
          (:`then_1`
            (`ActorComponent.K2_DestroyComponent` (`self.PotionC`)))
          (:`then_2`
            (bind _returnvalue_2 (`GameplayStatics.SpawnEmitterAtLocation` "/Game/StarterContent/Particles/P_Smoke.P_Smoke" _location (struct) (1.0 1.0 1.0) false))
            (`KismetSystemLibrary.Delay` 1.5)
            (`ActorComponent.K2_DestroyComponent` _returnvalue_2)))))))

(event `self.PotionC.OnComponentHit`
  (params (HitComponent :type "PrimitiveComponent Object Reference") (OtherActor :type "Actor Object Reference") (OtherComp :type "PrimitiveComponent Object Reference") (NormalImpulse :type "Vector Structure") (Hit :type "HitResult Structure (by ref)")))

(fn `UserConstructionScript`)